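; Player Blueprint for the Drifter, handling warmth as a survival meter, bullet time, checkpoints and timed invincibility.
; Q or left mouse slows global time with compensated custom dilation and a material parameter collection fade, against a draining, refilling meter.
; Warmth timeline counts down to death and the loss widget; Win stops it.
; Checkpoint overlaps save warmth, which resets lerp back to; Space plays character sound.
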(event `self.ReceiveBeginPlay`
  (bind _maxwarm (`self.MaxWarm`))
  (set `self.BulletTimeState` (`self.MaxBulletTime`))
  (set `self.Warm` _maxwarm)
  (set `self.LastWarm` _maxwarm)
  (`TimelineComponent.SetTimelineLength` (`self.ActivateInvincible`) (`self.InvincibleTime`)))

(event `self.ReceiveActorBeginOverlap`
  (params (OtherActor :type "Actor Object Reference"))
  (bind _ascheck_point (cast `CheckPoint` OtherActor))
  (if (`CheckPoint.Active` _ascheck_point)
    (`CheckPoint.Disable` _ascheck_point)
    (set `self.LastCheckPoint` _ascheck_point)
    (set `self.LastWarm` (`self.Warm`))
    (`KismetSystemLibrary.PrintString` "CheckPoint Saved")))

(event `Key|SpaceBar`
  (params (Key :type "Key Structure"))
  ;[1 1 1] Making Sound during space bar pressing (character sound)
  (:`Pressed`
    (if (not (`AudioComponent.IsPlaying` (stale _returnvalue)))
      (`GameplayStatics.PlaySound2D` null 1.0 1.0 0.0 null null false)
      (bind _returnvalue (`AddComponent|NODE_AddAudioComponent-2`)))))

(event `Key|Q`
  (params (Key :type "Key Structure"))
  (:`Pressed`
    (if (> (`self.BulletTimeState`) 0.0) :!label _label
      (`self.BulletTimeUpdate` true)))
  (:`Released`
    (`self.BulletTimeUpdate` false :!label _label_2)))

(event `Key|LeftMouseButton`
  (params (Key :type "Key Structure"))
  (:`Pressed`
    (goto _label))
  (:`Released`
    (goto _label_2)))

(event `BulletTimeUpdate`
  (params (_inBulletTime :type Boolean))
  (bind _slowdown (`self.SlowDown`))
  (bind _output_get (set `self.InBulletTime` _inBulletTime))
  (if _output_get
    (`GameplayStatics.SetGlobalTimeDilation` _slowdown)
    (set `self.CustomTimeDilation` (/ 0.6 _slowdown))
    (bind (_direction _mpc_alpha) (`Timeline|VFXFade` :!label _label_3)
      (:`Update`
        (`KismetMaterialLibrary.SetScalarParameterValue` "/Game/Materials/MPC_BulletTime.MPC_BulletTime" "Alpha" _mpc_alpha)))
    (else
      (`GameplayStatics.SetGlobalTimeDilation` 1.0)
      (set `self.CustomTimeDilation` 1.0)
      (goto _label_3 :!via `Reverse`))))

(event `BecomeInvincible`
  (set `self.Invincible` true)
  (`Timeline|ActivateInvincible` :!via `PlayFromStart`
    (:`Finished`
      (set `self.Invincible` false))))

(event `self.OnResetFinished`
  (set `self.Warm` (`self.LastWarm`))
  (`KismetSystemLibrary.PrintString` "Reset"))

(event `self.OnResetStart`
  (bind _resettimeline (`self.ResetTimeLine`))
  ;[0.2087 1 0.7254] Naive Reset
  (`TimelineComponent.SetTimelineLength` _resettimeline (`self.ResetTime`))
  (`Timeline|ResetTimeline` :!via `PlayFromStart`
    (:`Update`
      (set `self.Warm` (`KismetMathLibrary.Lerp` (`self.Warm`) (`self.LastWarm`) (/ (`TimelineComponent.GetPlaybackPosition` _resettimeline) (`TimelineComponent.GetTimelineLength` _resettimeline)))))
    (:`Finished`
      (`self.ResetInternal`)
      (`self.OnResetFinished`)
      (`TimelineComponent.Play` (`self.Warmth`)))))

(fn `UserConstructionScript`)

(fn `Win`
  (`TimelineComponent.Stop` (`self.Warmth`)))
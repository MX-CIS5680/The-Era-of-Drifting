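; Checkpoint actor Blueprint that animates the emissive glow of its mesh while it is not active.
; BeginPlay gives the mesh a dynamic material instance, and Tick plays a color timeline whenever IsActive is false.
; The timeline drives the material's emissive color and brightness parameters.
; The overlap and DisableEffect events are empty, so this graph holds no trigger or activation logic.
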(event `self.ReceiveBeginPlay`
  (bind _mesh (`self.Mesh`))
  (bind _returnvalue (`KismetMaterialLibrary.CreateDynamicMaterialInstance` (`PrimitiveComponent.GetMaterial` _mesh 0)))
  (bind _output_get (set `self.D_MaterialRef` _returnvalue))
  (`PrimitiveComponent.SetMaterial` _mesh 0 _output_get))

(event `self.ReceiveTick`
  (params (DeltaSeconds :type "Float (single-precision)"))
  (bind _mesh (`self.Mesh`))
  (if (not (`self.IsActive`))
    (bind (_direction _color _emission) (`Timeline|LerpColorTimeLine`)
      (:`Update`
        (`MeshComponent.SetVectorParameterValueOnMaterials` _mesh "Emiss_Color" (`KismetMathLibrary.Conv_LinearColorToVector` _color))
        (`MeshComponent.SetScalarParameterValueOnMaterials` _mesh "Emiss_Brightness" _emission)))))

(event `self.DisableEffect`)

(fn `UserConstructionScript`)
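; BP_RewindPlayer drives the rewind and reset effect for the BP_Drifter player pawn, which it caches on BeginPlay.
; StartResetDelay plays the SlowDown timeline, which raises the gray screen alpha and lowers time dilation, then restores time and starts the drifter's reset.
; During rewind playback it feeds the rewind percent into the drifter's warm lerp.
; When the sequence player finishes, it briefly waits, ends the rewind and notifies the drifter.
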(event `self.ReceiveBeginPlay`
  (bind _asbp_drifter (cast `/Game/Blueprints/BP_Drifter` (`GameplayStatics.GetPlayerPawn` 0)))
  (set `self.BP_Player` _asbp_drifter))

(event `self.OnRewindStart`
  (`|ExecutionSequence`
    (:`then_1`
      (`/Engine/EditorBlueprintResources/StandardMacros.DoOnce` false
        (:`Completed`
          (add `MovieSceneSequencePlayer.OnFinished` (`self.SequencePlayer`) (delegate `OnFinished_Event`)))))))

(event `OnFinished_Event`
  (`KismetSystemLibrary.Delay` 0.1)
  (`self.EndRewind`)
  (`TheEraOfDriftingCharacter.OnResetFinished` (`self.BP_Player`)))

(event `self.ReceiveTick`
  (params (DeltaSeconds :type "Float (single-precision)")))

(event `self.OnRewindPlaying`
  (`/Game/Blueprints/BP_Drifter.LerpWarmByPer` (`self.BP_Player`) (`self.GetRewindPercent`)))

(fn `StartResetDelay`
  (`TimelineComponent.PlayFromStart` (`self.SlowDown`)))

(fn `UserConstructionScript`)
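; BP_RewindRecorder is an actor that manages the lifecycle of a recording, named for a rewind feature.
; On BeginPlay it binds an end-play handler and plays a Timeline, starting the recording only when the Timeline finishes.
; Tick polls the game's pause state every frame to pause or resume recording.
; When play ends, it stops the recording and resets it.
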(event `self.ReceiveBeginPlay`
  (add `Actor.OnEndPlay` (delegate `OnEndPlay_Event`))
  (`Timeline|Timeline`
    (:`Finished`
      (`self.StartRecord`))))

(event `OnEndPlay_Event`
  (params (Actor :type "Actor Object Reference") (EndPlayReason :type "EEndPlayReason Enum" :default "Destroyed"))
  (`self.StopRecord`)
  (`self.ResetForRecord`))

(event `self.ReceiveTick`
  (params (DeltaSeconds :type "Float (single-precision)"))
  (if (`GameplayStatics.IsGamePaused`)
    (`self.PauseRecord`)
    (else
      (`self.ResumeRecord`))))

(fn `UserConstructionScript`)
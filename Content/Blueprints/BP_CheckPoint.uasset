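; Checkpoint actor that points a particle effect toward a Target and changes its mesh's glow.
; BeginPlay puts a dynamic material on the mesh.
; On Tick, DoOnce gates set the effect's ForceDir toward Target while IsActive is true; otherwise they activate the effect, play audio and start the color change.
; A timeline drives the material's emissive color and brightness; DisableEffect is an empty stub.
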(event `self.ReceiveBeginPlay`
  (bind _mesh (`self.Mesh`))
  (`SceneComponent.K2_AttachToComponent` (`self.PointToEffect`) (`self.RootComponent`) "None" "KeepRelative" "KeepWorld" "KeepRelative" true)
  (bind _returnvalue (`KismetMaterialLibrary.CreateDynamicMaterialInstance` (`PrimitiveComponent.GetMaterial` _mesh 0)))
  (bind _output_get (set `self.D_MaterialRef` _returnvalue))
  (`PrimitiveComponent.SetMaterial` _mesh 0 _output_get))

(event `self.ReceiveTick`
  (params (DeltaSeconds :type "Float (single-precision)"))
  (bind _mesh (`self.Mesh`))
  (if (`self.IsActive`)
    (`/Engine/EditorBlueprintResources/StandardMacros.DoOnce` false
      (:`Completed`
        (if (`KismetSystemLibrary.IsValid` (`self.Target`))
          (`NiagaraComponent.SetVariableVec3` (`self.PointToEffect`) "ForceDir" (* (`self.PointToLength`) (`KismetMathLibrary.Normal` (- (`self.K2_GetActorLocation` (`self.Target`)) (`self.K2_GetActorLocation`))))))))
    (else
      (`|ExecutionSequence`
        (:`then_0`
          (if (`KismetSystemLibrary.IsValid` (`self.Target`))
            (`/Engine/EditorBlueprintResources/StandardMacros.DoOnce` false
              (:`Completed`
                (`ActorComponent.SetActive` (`self.PointToEffect`) true false)))))
        (:`then_1`
          (`/Engine/EditorBlueprintResources/StandardMacros.DoOnce` false
            (:`Completed`
              (`GameplayStatics.PlaySound2D` null 1.0 1.0 0.0 null null)
              (`AddComponent|NODE_AddAudioComponent-0`)
              (bind (_direction _color _emission) (`Timeline|LerpColorTimeLine`)
                (:`Update`
                  (`MeshComponent.SetVectorParameterValueOnMaterials` _mesh "Emiss_Color" (`KismetMathLibrary.Conv_LinearColorToVector` _color))
                  (`MeshComponent.SetScalarParameterValueOnMaterials` _mesh "Emiss_Brightness" _emission))))))))))

(event `self.DisableEffect`)

(fn `UserConstructionScript`)
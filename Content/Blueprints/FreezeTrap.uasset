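; Trap actor that freezes a BP_Drifter touching it and shows an ice mesh at the drifter's location.
; Begin overlap and a per-tick box collider check both call TryFreeze, which skips invincible drifters and sets a Triggered lock.
; The InFreeze timeline serves as a FreezeTime-length timer.
; When it finishes, it unfreezes the begin-overlap drifter with invincibility, hides the ice and re-arms the trap.
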(event `self.ReceiveBeginPlay`
  (`TimelineComponent.SetTimelineLength` (`self.InFreeze`) (`self.FreezeTime`)))

(event `self.ReceiveActorBeginOverlap`
  (params (OtherActor :type "Actor Object Reference"))
  (if (not (`self.Triggered`))
    (bind _asbp_drifter (cast `/Game/Blueprints/BP_Drifter` OtherActor))
    (`self.TryFreeze` _asbp_drifter)))

(event `self.ReceiveTick`
  (params (DeltaSeconds :type "Float (single-precision)"))
  (if (not (`self.Triggered`))
    (for _array_element (`PrimitiveComponent.GetOverlappingActors` (`self.BoxCollider`) null)
      (bind _asbp_drifter (cast `/Game/Blueprints/BP_Drifter` _array_element))
      (`self.TryFreeze` _asbp_drifter))))

(fn `FreezeEffect`
  (params (PlayerLocation :type "Vector Structure"))
  (bind _ice (`self.Ice`))
  (`SceneComponent.K2_SetWorldLocation` _ice PlayerLocation false false)
  (`SceneComponent.SetHiddenInGame` _ice false false))

(fn `TryFreeze`
  (params (drifter :type "/Game/Blueprints/BP_Drifter Object Reference"))
  (if (not (`/Game/Blueprints/BP_Drifter.Invincible` drifter))
    (`TheEraOfDriftingCharacter.Freeze` drifter)
    (`self.FreezeEffect` (`self.K2_GetActorLocation` drifter))
    (set `self.Triggered` true)
    (`KismetSystemLibrary.PrintString` "Freeze")
    (`TimelineComponent.PlayFromStart` (`self.InFreeze`))))

(fn `UserConstructionScript`)
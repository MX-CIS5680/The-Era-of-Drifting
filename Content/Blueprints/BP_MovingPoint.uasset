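; BP_MovingPoint is an actor that uses an InterpToMovement component to move along a path whose end is defined by a Cube component.
; The construction script seeds two relative control points at zero offset.
; When the movement component activates, it overwrites the second point with the Cube's relative location and hides the Cube, which thus serves as a destination marker.
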(event `self.ReceiveBeginPlay`)

(event `self.InterpToMovement.OnComponentActivated`
  (params (Component :type "ActorComponent Object Reference") (bReset :type Boolean))
  (bind _cube (`self.Cube`))
  (bind _returnvalue_location (`KismetMathLibrary.BreakTransform` (`SceneComponent.GetRelativeTransform` _cube)))
  (bind _asinterp_to_movement_component (cast `InterpToMovementComponent` Component))
  (`|VariableSetRef` (`|GetArrayItem` (`InterpToMovementComponent.ControlPoints` _asinterp_to_movement_component) 1) (make `InterpControlPoint` _returnvalue_location))
  (`SceneComponent.SetVisibility` _cube false false))

(fn `UserConstructionScript`
  (`InterpToMovementComponent.AddControlPointPosition` (`self.InterpToMovement`) (0.0 0.0 0.0) true)
  (`InterpToMovementComponent.AddControlPointPosition` (`self.InterpToMovement`) (0.0 0.0 0.0) true))